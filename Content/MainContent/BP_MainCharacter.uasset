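; BP_MainCharacter is the player character, handling axis-driven walking and strafing, mouse look, and interaction with actors in view.
; On Interact, GetViewPoint and GetTraceData derive a trace from the controller's view point, scaled by InteractDistance.
; MakeTrace runs a Visibility line trace with timed debug drawing, then InteractWithActor sends InteractMessage to a hit actor implementing the interact interface, passing itself.
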(event Input|ActionEvents|InputActionInteract
  (params (Key :type Key%20Structure :default "None"))
  (bind (_success _tracestart _traceend) (CallFunction|GetTraceData))
  ;[1 1 1] Interaction
  (:Pressed
    (if _success
      (bind _hitresult (CallFunction|MakeTrace _tracestart _traceend))
      (CallFunction|InteractwithActor _hitresult))))

(event Input|AxisEvents|InputAxisMoveForward
  (params (AxisValue :type Float%20%28single-precision%29))
  ;[1 1 1] Movement
  (Pawn|Input|AddMovementInput (Transformation|GetActorForwardVector) AxisValue false))

(event Input|AxisEvents|InputAxisMoveRight
  (params (AxisValue :type Float%20%28single-precision%29))
  ;[1 1 1] Movement
  (Pawn|Input|AddMovementInput (Transformation|GetActorRightVector) AxisValue false))

(event Input|MouseEvents|MouseX
  (params (AxisValue :type Float%20%28single-precision%29))
  ;[1 1 1] Turning
  (Pawn|Input|AddControllerYawInput AxisValue))

(event Input|MouseEvents|MouseY
  (params (AxisValue :type Float%20%28single-precision%29))
  ;[1 1 1] Turning
  (Pawn|Input|AddControllerPitchInput AxisValue))

(fn ConstructionScript)

(fn MakeTrace
  (params (TraceStart :type Vector) (TraceEnd :type Vector))
  (bind _outhit (Collision|LineTraceByChannel TraceStart TraceEnd "TraceTypeQuery1" false 0 "ForDuration" true "(R=1.000000,G=0.000000,B=0.000000,A=1.000000)" "(R=0.000000,G=1.000000,B=0.000000,A=1.000000)" 2.0))
  (return _outhit))

(fn GetViewPoint
  (bind _returnvalue (Pawn|GetController))
  (bind (_location _rotation) (Pawn|GetPlayerViewPoint _returnvalue))
  (Utilities|IsValid _returnvalue
    (:Is%20Valid
      (return true _location _rotation))
    (:Is%20Not%20Valid
      (return false "0, 0, 0" "0, 0, 0"))))

(fn GetTraceData
  (bind (_success _viewlocation _viewrotation) (CallFunction|GetViewPoint))
  (if _success
    (return true _viewlocation (+ _viewlocation (* _viewrotation (Variables|Interact|GetInteractDistance))))
    (else
      (return false "0, 0, 0" "0, 0, 0"))))

(fn InteractwithActor
  (params (HitResult :type Hit%20Result%20Structure%20%28by%20ref%29))
  (bind (_bblockinghit _binitialoverlap _time _distance _location _impactpoint _normal _impactnormal _physmat _hitactor) (Collision|BreakHitResult HitResult))
  (if _bblockinghit
    (Utilities|IsValid _hitactor
      (:Is%20Valid
        (if (Utilities|DoesObjectImplementInterface _hitactor (LocalVariables|GetInteractInterfaceClass))
          (Class|BPIInteract|Interact(Message) _hitactor self))))))