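; Interactable URL-entry actor that lets a player enter an address and send it to linked terminals.
; Interacting focuses the player's pawn on the WURL widget component and creates the user widget for that pawn's controller.
; Clicking the search button mesh block-loads each referenced terminal, reads the URL from WBP_URL, and calls LoadSite on that BP_Terminal.
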(event OnClicked(SM_SearchButton)
  (params (TouchedComponent :type Primitive%20Component%20Object%20Reference) (ButtonPressed :type Key%20Structure :default "None"))
  (bind (_success _url) (CallFunction|GetWidgetURL))
  ;[1 1 1] On Clicket SearchButton
  (for _array_element (Variables|Default|GetTerminalActors)
    (bind _returnvalue (Utilities|LoadAssetBlocking _array_element))
    (bind _asbp_terminal (Utilities|Casting|CastToBP_Terminal _returnvalue))
    (if _success
      (Default|LoadSite _asbp_terminal (Utilities|String|ToString(Text) _url)))))

(event EventInteract
  (params (InteractingActor :type Actor%20Object%20Reference))
  ;[1 1 1] Interact Event
  (bind _aspawn (Utilities|Casting|CastToPawn InteractingActor))
  (CallFunction|FocusPlayer _aspawn (Variables|Default|GetW_URL))
  (Utilities|IsValid (Pawn|GetController _aspawn)
    (:Is%20Valid
      (CallFunction|CreateUserWidget (Pawn|GetController _aspawn)))))

(fn ConstructionScript)

(fn GetWidgetURL
  (bind _w_url (Variables|Default|GetW_URL))
  (bind _returnvalue (UserInterface|GetUserWidgetObject _w_url))
  (Utilities|IsValid _w_url
    (:Is%20Valid
      (Utilities|IsValid _returnvalue
        (:Is%20Valid
          (bind _aswbp_url (Utilities|Casting|CastToWBP_URL _returnvalue)
            (:then
              (bind _returnvalue_2 (Default|GetURL _aswbp_url))
              (return true _returnvalue_2))
            (:CastFailed
              _)))
        (:Is%20Not%20Valid
          _)))
    (:Is%20Not%20Valid
      _))
  (return false ""))