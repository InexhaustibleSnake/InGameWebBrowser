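; Interactable computer terminal with a world-space web browser screen and a clickable power button.
; On interact it focuses the pawn on the screen widget and creates a user widget for its controller.
; The power button toggles Enabled, swapping its material, showing or hiding the screen and resetting the browser; LoadSite passes a URL to WBP_WebBrowser.
; FocusPlayerOnScreen and CalculateNewPlayerRotation hold only disconnected logic.
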(event OnClicked(SM_PowerButton)
  (params (TouchedComponent :type Primitive%20Component%20Object%20Reference) (ButtonPressed :type Key%20Structure :default "None"))
  ;[1 1 1] On Power Button Clicked
  (Variables|Default|SetEnabled (not (Variables|Default|GetEnabled)))
  (CallFunction|ChangePowerButtonMaterial)
  (CallFunction|SetScreenVisibility)
  (CallFunction|ResetBrowser))

(event Custom|LoadSite
  (params (SiteURL :type String))
  ;[1 1 1] Load Site
  (bind _aswbp_web_browser (Utilities|Casting|CastToWBP_WebBrowser (UserInterface|GetUserWidgetObject (Variables|Default|GetW_Screen))))
  (Default|LoadURL _aswbp_web_browser SiteURL))

(event EventInteract
  (params (InteractingActor :type Actor%20Object%20Reference))
  ;[1 1 1] Event Interact
  (bind _aspawn (Utilities|Casting|CastToPawn InteractingActor))
  (CallFunction|FocusPlayer _aspawn (Variables|Default|GetW_Screen))
  (Utilities|IsValid (Pawn|GetController _aspawn)
    (:Is%20Valid
      (CallFunction|CreateUserWidget (Pawn|GetController _aspawn)))))

(event EventBeginPlay
  ;[1 1 1] Begin Play
  (CallFunction|SetScreenVisibility))

(fn ConstructionScript)

(fn FocusPlayeronScreen
  (params (PlayerController :type Player%20Controller%20Object%20Reference)))

(fn ChangePowerButtonMaterial
  (Rendering|Material|SetMaterial (Variables|Default|GetSM_PowerButton) 0 (select (Variables|Default|GetEnabled) (Variables|PowerButton|GetPowerButtonOnMaterial) (Variables|PowerButton|GetPowerButtonOffMaterial))))

(fn SetScreenVisibility
  (Widget|SetVisibility (UserInterface|GetUserWidgetObject (Variables|Default|GetW_Screen)) (select (Variables|Default|GetEnabled) "Visible" "Hidden")))

(fn ResetBrowser
  (bind _aswbp_web_browser (Utilities|Casting|CastToWBP_WebBrowser (UserInterface|GetWidget (Variables|Default|GetW_Screen))))
  (Default|ResetBrowser _aswbp_web_browser))

(fn ChangePlayerMovement
  (params (PlayerCharacter :type Character%20Object%20Reference))
  (bind _charactermovement (Variables|/Script/Engine.Character|GetCharacterMovement PlayerCharacter))
  (Utilities|IsValid PlayerCharacter
    (:Is%20Valid
      (Utilities|IsValid _charactermovement
        (:Is%20Valid
          (Pawn|Components|CharacterMovement|SetMovementMode _charactermovement "MOVE_None" 0))))))