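; Base interactible Blueprint that provides an empty Interact event and shared helpers for showing and focusing interaction UI.
; CreateUserWidget spawns the configured InteractWidgetClass for a given player controller and adds it to the viewport.
; FocusPlayer takes a widget component, switches the player to Game and UI input focused on its widget with mouse lock, shows the cursor and disables pawn input.
; The file contains no logic to restore input.
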(event EventInteract
  (params (InteractingActor :type Actor%20Object%20Reference)))

(fn ConstructionScript)

(fn FocusPlayer
  (params (PlayerPawn :type Pawn%20Object%20Reference) (WidgetToFocus :type Widget%20Component%20Object%20Reference))
  (bind _returnvalue (Pawn|GetController PlayerPawn))
  (bind _returnvalue_2 (UserInterface|GetUserWidgetObject WidgetToFocus))
  (Utilities|IsValid _returnvalue
    (:Is%20Valid
      (bind _asplayer_controller (Utilities|Casting|CastToPlayerController _returnvalue))
      (LocalVariables|SetPlayerController _asplayer_controller)
      (Utilities|IsValid WidgetToFocus
        (:Is%20Valid
          (Utilities|IsValid _returnvalue_2
            (:Is%20Valid
              (Input|SetInputModeGameandUI (LocalVariables|GetPlayerController) _returnvalue_2 "LockAlways" true false)
              (Variables|/Script/Engine.PlayerController|SetbShowMouseCursor (LocalVariables|GetPlayerController) true)
              (Input|DisableInput (Pawn|GetControlledPawn (LocalVariables|GetPlayerController)) (LocalVariables|GetPlayerController)))))))))

(fn CreateUserWidget
  (params (Controller :type Controller%20Object%20Reference))
  (if (Utilities|IsValidClass (Variables|Default|GetInteractWidgetClass))
    (Utilities|IsValid Controller
      (:Is%20Valid
        (bind _asplayer_controller (Utilities|Casting|CastToPlayerController Controller))
        (bind _returnvalue (UserInterface|CreateWidget (Variables|Default|GetInteractWidgetClass) _asplayer_controller))
        (Utilities|IsValid _returnvalue
          (:Is%20Valid
            (UserInterface|Viewport|AddtoViewport _returnvalue 0)))))))